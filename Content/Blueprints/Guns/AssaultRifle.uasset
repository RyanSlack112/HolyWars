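; Player assault rifle with automatic hitscan fire, toggle or hold aim-down-sights via camera FOV, and delayed reload standing in for an animation.
; FireGun re-arms itself on a fire-rate timer, and each line trace reports gunfire and impact noise, plus a damage event on Guard hits.
; Spread grows multiplicatively per shot up to a cap, decays on a looping timer, and resets on holster.
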(event EventFireReleased
  (params (FiringTransform :type Transform))
  ;[1 1 1] Event Fire Released
  (Variables|Default|SetCanFire false))

(event EventHolster
  ;[1 1 1] Event Holster
  (Utilities|Time|ClearTimerbyFunctionName 0 "FireGun")
  (Utilities|Time|ClearTimerbyFunctionName 0 "DecreaseSpread")
  (Variables|Stats|SetSpread 0.0)
  (if (Variables|Default|GetAiming)
    (Variables|Default|SetAiming false)
    (Default|ChangeFieldOfView (Variables|Default|GetCharacter) 9e+01 0.0)))

(event EventReload
  ;[1 1 1] Event Reload
  (Utilities|ReloadRifle))

(event EventFirePressed
  (params (FiringTransform :type Transform))
  ;[1 1 1] Event Fire Pressed
  (Variables|Default|SetCanFire true)
  (if (not (Class|KismetSystemLibrary|TimerExists 0 "FireGun"))
    (CallFunction|FireGun)))

(event EventAltFirePressed
  (bind _character (Variables|Default|GetCharacter))
  ;[1 1 1] Event Alt Fire Pressed
  (if (Variables|Default|GetAimToggle)
    (bind _output_get (Variables|Default|SetAiming (not (Variables|Default|GetAiming))))
    (if _output_get
      (Default|ChangeFieldOfView _character 4e+01 0.05)
      (else
        (Default|ChangeFieldOfView _character 9e+01 0.05)))
    (else
      (Variables|Default|SetAiming true)
      (Default|ChangeFieldOfView (Variables|Default|GetCharacter) 4e+01 0.05))))

(event EventAltFireReleased
  ;[1 1 1] Event Alt Fire Released
  (if (not (Variables|Default|GetAimToggle))
    (Variables|Default|SetAiming false)
    (Default|ChangeFieldOfView (Variables|Default|GetCharacter) 9e+01 0.05)))

(fn ConstructionScript)

(fn FireGun
  (if (Math|Boolean|ANDBoolean (> (Variables|Default|GetCurrentMagazineSize) 0) (Variables|Default|GetCanFire) (not (Variables|Default|GetReloading)))
    (CallFunction|FireBullet (Transformation|GetWorldTransform (Variables|/Game/Blueprints/Characters/Characters/BaseCharacter/BaseCharacter.BaseCharacter_C|GetCamera (Variables|Default|GetCharacter))))
    (CallFunction|IncreaseSpread)
    (if (Class|KismetSystemLibrary|TimerExists 0 "DecreaseSpread")
      _
      (else
        (CallFunction|DecreaseSpread) ; Decrease spread at a constant rate
        (Utilities|Time|SetTimerbyFunctionName 0 "DecreaseSpread" (Variables|Stats|GetSpreadDecreaseRate) true)))
    (Utilities|Time|SetTimerbyFunctionName self "FireGun" (Variables|Default|GetFireRate)) ; FireRate cooldown
  ))

(fn FireBullet
  (params (FiringTransform :type Transform))
  (bind _returnvalue (Game|GetInstigator))
  (bind _returnvalue_2 (Transformation|GetActorLocation))
  (bind (_start _end) (|GetStartandEndLineTraceLocations FiringTransform))
  (Development|PrintString "Pew")
  (Math|Integer|DecrementInt (Variables|Default|GetCurrentMagazineSize)
    (:%20%20
      (bind _outhit (Collision|LineTraceByChannel _start _end "TraceTypeQuery4" false 0 "ForDuration" true "(R=1.000000,G=0.000000,B=0.000000,A=1.000000)" "(R=0.000000,G=0.201691,B=1.000000,A=1.000000)"))
      ;[1 1 1] Noise Events
      (Class|AISenseHearing|ReportNoiseEvent (.location _outhit) 1.0 _returnvalue 5e+02 "BulletCollision")
      (Class|AISenseHearing|ReportNoiseEvent _returnvalue_2 1.0 _returnvalue 1e+03 "GunFire")
      (bind _asguard (Utilities|Casting|CastToGuard (.hitactor _outhit)))
      ;[1 1 1] Damage Event
      (Class|AISenseDamage|ReportDamageEvent _asguard _returnvalue (Math|Conversions|ToFloat(Integer) (Variables|Default|GetDamage)) _returnvalue_2 (.location _outhit)))))

(fn DecreaseSpread
  (bind _output_get (Variables|Stats|SetSpread (Math|Float|Max(Float) (- (Variables|Stats|GetSpread) (Variables|Stats|GetSpreadDecrease)) 0.0)))
  (if (<= _output_get 0.0)
    (Utilities|Time|ClearTimerbyFunctionName self "DecreaseSpread")))

(fn IncreaseSpread
  (if (== (Variables|Stats|GetSpread) 0.0)
    (Variables|Stats|SetSpread 1.0)
    (else
      (Variables|Stats|SetSpread (Math|Float|Min(Float) (* (Variables|Stats|GetSpread) (+ (/ (Variables|Stats|GetSpreadIncrease) 1e+02) 1.0)) (Variables|Stats|GetMaxSpread))))))