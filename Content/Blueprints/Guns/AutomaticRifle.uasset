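; Automatic rifle that fires hitscan shots repeatedly while fire is held, it is equipped and the magazine has rounds.
; A cooldown timer re-calls FireGun, and each shot raises a capped spread value that a looping timer decays.
; Line traces report impact and gunshot noise events, plus damage events on Guard hits, for AI senses.
; Reload refills the magazine from reserve ammo after a delay standing in for an animation.
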(event EventFireReleased
  (params (FiringTransform :type Transform))
  ;[1 1 1] Event Fire Released
  (Variables|Default|SetIsFiring false))

(event EventReload
  ;[1 1 1] Event Reload
  (Utilities|ReloadRifle))

(event EventFirePressed
  (params (FiringTransform :type Transform))
  ;[1 1 1] Event Fire Pressed
  (Variables|Default|SetIsFiring true)
  (CallFunction|FireGun))

(fn ConstructionScript)

(fn FireCoolDown
  (Variables|Default|SetCanFire true)
  (CallFunction|FireGun))

(fn FireGun
  (if (Math|Boolean|ANDBoolean (== (Variables|/Game/Blueprints/Characters/Characters/BaseCharacter/BaseCharacter.BaseCharacter_C|GetEquippedWeapon (Variables|Default|GetCharacter)) self) (> (Variables|Default|GetCurrentMagazineSize) 0) (Variables|Default|GetCanFire) (Variables|Default|GetIsFiring))
    (Variables|Default|SetCanFire false)
    (Variables|Default|SetFiringTransform (Transformation|GetWorldTransform (Variables|/Game/Blueprints/Characters/Characters/BaseCharacter/BaseCharacter.BaseCharacter_C|GetCamera (Variables|Default|GetCharacter))))
    (CallFunction|FireBullet)
    (Variables|Stats|SetSpread (Math|Float|Min(Float) (+ (Variables|Stats|GetSpread) (Variables|Stats|GetSpreadIncrease)) (Variables|Stats|GetMaxSpread))) ; Increases Spread
    (Utilities|Time|SetTimerbyFunctionName 0 "DecreaseSpread" 0.1 true) ; Decreases spread at a constant rate
    (Utilities|Time|SetTimerbyFunctionName 0 "FireCoolDown" (Variables|Default|GetFireRate)) ; After a period of time, set CanFire back to true and fire again
  ))

(fn FireBullet
  (bind _returnvalue (Game|GetInstigator))
  (bind _returnvalue_2 (Transformation|GetActorLocation))
  (bind (_start _end) (|GetStartandEndLineTraceLocations))
  (Math|Integer|DecrementInt (Variables|Default|GetCurrentMagazineSize)
    (:%20%20
      (bind _outhit (Collision|LineTraceByChannel _start _end "TraceTypeQuery4" false 0 "ForDuration" true "(R=1.000000,G=0.000000,B=0.000000,A=1.000000)" "(R=0.000000,G=0.201691,B=1.000000,A=1.000000)"))
      ;[1 1 1] Noise Events
      (Class|AISenseHearing|ReportNoiseEvent (.location _outhit) 1.0 _returnvalue 5e+02 "BulletCollision")
      (Class|AISenseHearing|ReportNoiseEvent _returnvalue_2 1.0 _returnvalue 1e+03 "GunFire")
      (bind _asguard (Utilities|Casting|CastToGuard (.hitactor _outhit)))
      ;[1 1 1] Damage Event
      (Class|AISenseDamage|ReportDamageEvent _asguard _returnvalue (Math|Conversions|ToFloat(Integer) (Variables|Default|GetDamage)) _returnvalue_2 (.location _outhit)))))

(fn DecreaseSpread
  (bind _output_get (Variables|Stats|SetSpread (Math|Float|Max(Float) (- (Variables|Stats|GetSpread) 0.1) 0.0)))
  (if (<= _output_get 0.0)
    (Utilities|Time|ClearTimerbyFunctionName self "DecreaseSpread")))