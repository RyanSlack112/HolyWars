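; ThrowableSpear is a gun-style weapon Blueprint for a spear that is thrown as a projectile and can be recalled.
; Pressing fire, if not already thrown, spawns a SpearProjectile slightly ahead of and above the weapon, passes itself as a reference, and hides its own mesh hierarchy.
; Releasing alt fire while thrown tells that projectile to return to its owner.
; Nothing here resets the thrown state or visibility.
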(event EventAltFireReleased
  ;[1 1 1] Event Alt Fire
  (if (Variables|Default|GetIsThrown)
    (Default|ReturntoOwner (Variables|Default|GetSpearProjectile))))

(event EventFireReleased
  (params (FiringTransform :type Transform))
  ;[1 1 1] Event Fire Released
)

(event EventFirePressed
  (params (FiringTransform :type Transform))
  (bind _returnvalue (Game|GetInstigator))
  (bind _returnvalue_2 (Transformation|GetActorTransform))
  ;[1 1 1] Event Fire Pressed
  (if (not (Variables|Default|GetIsThrown))
    (Variables|Default|SetIsThrown true)
    (bind _returnvalue_3 (Game|SpawnActorfromClass "/Game/Blueprints/Projectiles/SpearProjectile.SpearProjectile_C" (Math|Transform|MakeTransform (+ (* (Math|Vector|GetForwardVector (.rotation FiringTransform)) 1e+02) (Math|Vector|MakeVector (.x (.location _returnvalue_2)) (.y (.location _returnvalue_2)) (+ (.z (.location _returnvalue_2)) 5e+01))) (.rotation FiringTransform) (.scale _returnvalue_2)) "AdjustIfPossibleButAlwaysSpawn" _returnvalue 2e+03 self _returnvalue))
    (Variables|Default|SetSpearProjectile _returnvalue_3)
    (Rendering|SetVisibility (Variables|Default|GetDefaultSceneRoot) false true)))

(fn ConstructionScript
  (|CallParentFunction))