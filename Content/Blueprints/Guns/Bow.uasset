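; Bow weapon that charges arrow speed while fire is held and launches an arrow projectile on release.
; A looping timer raises the speed until it reaches the bow's maximum.
; Release clears the timer and spawns the arrow just ahead of the bow with that speed.
; A camera line trace sets the arrow's rotation toward the hit point, or a far point if nothing is hit.
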(event Custom|IncreaseBowPower
  ;[1 1 1] Increase Bow Power
  (if (< (Variables|Default|GetArrowSpeed) (Variables|Default|GetMaxBowSpeed))
    (Variables|Default|SetArrowSpeed (+ (Variables|Default|GetArrowSpeed) 1e+02))
    (else
      (Utilities|Time|ClearandInvalidateTimerbyHandle (stale EventFirePressed _returnvalue)))))

(event EventFirePressed
  (params (FiringTransform :type Transform))
  ;[1 1 1] Event Fire Pressed. Charges Arrow power
  (Development|PrintString "Bow FirePressed")
  (Variables|Default|SetArrowSpeed 5e+02)
  (bind _returnvalue (Utilities|Time|SetTimerbyEvent (delegate Custom|IncreaseBowPower) 0.05 true)))

(event EventFireReleased
  (params (FiringTransform :type Transform))
  (bind _returnvalue (Transformation|GetActorLocation))
  (bind _arrowspeed (Variables|Default|GetArrowSpeed))
  ;[1 1 1] Event Fire Released, Releases Arrow
  (Utilities|Time|ClearTimerbyFunctionName self "IncreaseBowPower")
  (Game|SpawnActorfromClass "/Game/Blueprints/Projectiles/ArrowProjectile.ArrowProjectile_C" (Math|Transform|MakeTransform (CallFunction|GetDistantLocation _returnvalue (.rotation FiringTransform) 75.0) (CallFunction|GetProjectileRotation _returnvalue (.location FiringTransform) (.rotation FiringTransform) 5e+02)) "AdjustIfPossibleButAlwaysSpawn" 0 _arrowspeed (Game|GetInstigator))
  (Development|PrintString (Utilities|String|Append "Bow Power: " (Utilities|String|ToString(Float) _arrowspeed))))

(fn ConstructionScript)

(fn GetDistantLocation
  (params (CurrentLocation :type Vector) (CurrentRotation :type Rotator) (Distance :type Float%20%28single-precision%29))
  (return (+ CurrentLocation (* (Math|Vector|GetForwardVector CurrentRotation) Distance))))

(fn GetProjectileRotation
  (params (SpawnLocation :type Vector) (CameraLocation :type Vector) (CameraRotation :type Rotator) (Distance :type Float%20%28single-precision%29))
  (LocalVariables|SetLSpawnLocation SpawnLocation)
  (LocalVariables|SetLCameraLocation CameraLocation)
  (LocalVariables|SetLCameraRotation CameraRotation)
  (LocalVariables|SetLDistance Distance)
  (bind _output_get (LocalVariables|SetLongDistanceLocation (CallFunction|GetDistantLocation (LocalVariables|GetLCameraLocation) (LocalVariables|GetLCameraRotation) 5e+03)))
  (bind (_outhit _returnvalue) (Collision|LineTraceByChannel (LocalVariables|GetLCameraLocation) _output_get "TraceTypeQuery4" false 0 "None" true "(R=0.000000,G=0.292413,B=1.000000,A=1.000000)"))
  (if _returnvalue ; Check if there's an obstruction within distance specificed
    (return (Math|Rotator|FindLookatRotation (LocalVariables|GetLSpawnLocation) (.location _outhit))) ; If there is, set rotation towards said target
    (else
      (return (Math|Rotator|FindLookatRotation (LocalVariables|GetLSpawnLocation) (LocalVariables|GetLongDistanceLocation))) ; If not, set rotation towards arbitrarily far away location
    )))