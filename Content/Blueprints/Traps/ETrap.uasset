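; ETrap is a defusable trap that arms like a mine, clicking when stepped on and exploding when the overlap ends.
; Box begin overlap enables input for player controller 0, without filtering which actor entered.
; End overlap disables input and fires a RadialForce impulse with explosion effects, applying no damage.
; Pressing Interact while input is enabled destroys the Box and RadialForce components and plays smoke effects.
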(event OnComponentBeginOverlap(Box)
  (params (OverlappedComponent :type Primitive%20Component%20Object%20Reference) (OtherActor :type Actor%20Object%20Reference) (OtherComp :type Primitive%20Component%20Object%20Reference) (OtherBodyIndex :type Integer) (bFromSweep :type Boolean) (SweepResult :type Hit%20Result%20Structure%20%28by%20ref%29))
  (Input|EnableInput (Game|GetPlayerController 0))
  (Audio|PlaySoundatLocation "/Engine/VREditor/Sounds/UI/Click_on_Button.Click_on_Button" (Transformation|GetActorLocation) "0, 0, 0" 1.0 1.0 0.0 0 0 0))

(event OnComponentEndOverlap(Box)
  (params (OverlappedComponent :type Primitive%20Component%20Object%20Reference) (OtherActor :type Actor%20Object%20Reference) (OtherComp :type Primitive%20Component%20Object%20Reference) (OtherBodyIndex :type Integer))
  (bind _returnvalue (Transformation|GetActorLocation))
  (Input|DisableInput (Game|GetPlayerController 0))
  (Class|RadialForceComponent|FireImpulse (Variables|Default|GetRadialForce))
  (Audio|PlaySoundatLocation "/Game/StarterContent/Audio/Explosion01.Explosion01" _returnvalue "0, 0, 0" 1.0 1.0 0.0 0 0 0)
  (Effects|SpawnEmitteratLocation "/Game/StarterContent/Particles/P_Explosion.P_Explosion" _returnvalue))

(event Input|ActionEvents|InputActionInteract
  (params (Key :type Key%20Structure))
  (bind _returnvalue (Transformation|GetActorLocation))
  (:Pressed
    (Components|DestroyComponent (Variables|Default|GetBox))
    (Audio|PlaySoundatLocation "/Game/StarterContent/Audio/Smoke01.Smoke01" _returnvalue "0, 0, 0" 1.0 1.0 0.0 0 0 0)
    (Effects|SpawnEmitteratLocation "/Game/StarterContent/Particles/P_Smoke.P_Smoke" _returnvalue)))

(fn ConstructionScript)