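; A spotlight actor that calculates how brightly it lights the first-person character inside its box volume.
; Construction script applies the light settings and sizes the box to the cone's reach.
; Overlap updates the player's ActiveLights list and toggles a looping timer that recomputes Brightness from cone falloff, distance attenuation and intensity.
; The timer's Camera-channel trace starts and ends at the light's location, zeroing Brightness if it hits the player.
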(event OnComponentBeginOverlap(BoxCollision)
  (params (OverlappedComponent :type Primitive%20Component%20Object%20Reference) (OtherActor :type Actor%20Object%20Reference) (OtherComp :type Primitive%20Component%20Object%20Reference) (OtherBodyIndex :type Integer) (bFromSweep :type Boolean) (SweepResult :type Hit%20Result%20Structure%20%28by%20ref%29))
  (bind _self self)
  (bind _asfirst_person_character (Utilities|Casting|CastToFirstPersonCharacter OtherActor))
  (bind _output_get (Variables|Default|SetPlayer _asfirst_person_character))
  (Utilities|Array|AddUnique (Variables|/Game/Blueprints/Characters/FirstPersonCharacter/FirstPersonCharacter.FirstPersonCharacter_C|GetActiveLights _output_get) _self)
  (Utilities|Time|SetTimerbyFunctionName _self "GetCurrentLightOnPlayer" 0.2 true))

(event OnComponentEndOverlap(BoxCollision)
  (params (OverlappedComponent :type Primitive%20Component%20Object%20Reference) (OtherActor :type Actor%20Object%20Reference) (OtherComp :type Primitive%20Component%20Object%20Reference) (OtherBodyIndex :type Integer))
  (bind _self self)
  (bind _asfirst_person_character (Utilities|Casting|CastToFirstPersonCharacter OtherActor))
  (Utilities|Array|RemoveItem (Variables|/Game/Blueprints/Characters/FirstPersonCharacter/FirstPersonCharacter.FirstPersonCharacter_C|GetActiveLights _asfirst_person_character) _self)
  (Utilities|Time|ClearTimerbyFunctionName _self "GetCurrentLightOnPlayer")
  (Variables|Default|SetPlayer 0))

(event Custom|GetCurrentLightOnPlayer
  (bind _player (Variables|Default|GetPlayer))
  (bind _spotlight (Variables|Default|GetSpotLight))
  (bind _returnvalue (Transformation|GetDistanceTo _player))
  (bind _outerconeangle (Variables|/Script/Engine.SpotLightComponent|GetOuterConeAngle _spotlight))
  (bind _returnvalue_2 (Math|Trig|Cos(Degrees) _outerconeangle))
  (bind _outhit (Collision|LineTraceByChannel (Transformation|GetActorLocation) (Transformation|GetActorLocation) "TraceTypeQuery2" false 0 "ForDuration" true "(R=1.000000,G=0.000000,B=0.000000,A=1.000000)" "(R=0.000000,G=1.000000,B=0.000000,A=1.000000)" 1.0))
  (if (== (.hitactor _outhit) _player)
    (Variables|Default|SetBrightness 0.0)
    (else
      (Variables|Default|SetBrightness (* (|(pow((clamp(((DotProduct-CosOuterCone)*InvCosConeDif),0,1)),2)) (Math|Vector|DotProduct (Math|Vector|Normalize (- (Transformation|GetActorLocation) (Transformation|GetActorLocation _player))) (* (Math|Vector|GetForwardVector (Transformation|GetActorRotation)) -1.0)) _returnvalue_2 (|(1/(CosInner-CosOuter)) (Math|Trig|Cos(Degrees) (Variables|/Script/Engine.SpotLightComponent|GetInnerConeAngle _spotlight)) _returnvalue_2)) (|(numerator/((pow(distance,2))+1)) (|(pow((clamp((1-(pow((distance/radius),4))),0,1)),2)) _returnvalue (Variables|/Script/Engine.LocalLightComponent|GetAttenuationRadius _spotlight)) _returnvalue) (Variables|/Script/Engine.LightComponentBase|GetIntensity (Variables|Default|GetSpotLight)))))))

(fn ConstructionScript
  (Constructors|SetSpotLightParameters)
  (Constructors|SetBoxCollisionParameters))

(fn SetSpotLightParameters
  (bind _spotlight (Variables|Default|GetSpotLight))
  (bind _innerconeangle (Variables|LightConstruction|GetInnerConeAngle))
  (Rendering|Components|Light|SetIntensity _spotlight (Variables|LightConstruction|GetLightIntensity))
  (Rendering|Lighting|SetAttenuationRadius _spotlight (Variables|LightConstruction|GetLightAttenuationRadius))
  (Rendering|Lighting|SetInnerConeAngle _spotlight _innerconeangle)
  (bind _output_get (Variables|LightConstruction|SetOuterConeAngle (Math|Float|Max(Float) _innerconeangle (Variables|LightConstruction|GetOuterConeAngle))))
  (Rendering|Lighting|SetOuterConeAngle _spotlight _output_get))

(fn SetBoxCollisionParameters
  (bind _lightattenuationradius (Variables|LightConstruction|GetLightAttenuationRadius))
  (bind _outerconeangle (Variables|LightConstruction|GetOuterConeAngle))
  (bind _boxcollision (Variables|Default|GetBoxCollision))
  (bind _returnvalue (Math|Trig|Sin(Degrees) _outerconeangle))
  (bind _returnvalue_2 (/ _lightattenuationradius 2.0))
  (bind _returnvalue_3 (* _lightattenuationradius _returnvalue))
  (Transformation|SetRelativeLocation _boxcollision (Math|Vector|MakeVector _returnvalue_2 0.0 0.0) false false)
  (Components|Box|SetBoxExtent _boxcollision (Math|Vector|MakeVector _returnvalue_2 _returnvalue_3 _returnvalue_3) true))