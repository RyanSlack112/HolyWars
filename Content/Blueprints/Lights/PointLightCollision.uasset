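; A point light actor that measures how much light it casts on the first-person character, storing it as Brightness.
; The construction script configures the light and matches a collision sphere to its attenuation radius.
; Overlap adds or removes the light in the character's ActiveLights and starts or stops a looping timer.
; Each tick of that timer line-traces for occlusion, computes windowed inverse-square falloff times intensity, and prints unoccluded results.
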(event OnComponentBeginOverlap(LightCollision)
  (params (OverlappedComponent :type Primitive%20Component%20Object%20Reference) (OtherActor :type Actor%20Object%20Reference) (OtherComp :type Primitive%20Component%20Object%20Reference) (OtherBodyIndex :type Integer) (bFromSweep :type Boolean) (SweepResult :type Hit%20Result%20Structure%20%28by%20ref%29))
  (bind _asfirst_person_character (Utilities|Casting|CastToFirstPersonCharacter OtherActor))
  (Utilities|Array|AddUnique (Variables|/Game/Blueprints/Characters/FirstPersonCharacter/FirstPersonCharacter.FirstPersonCharacter_C|GetActiveLights _asfirst_person_character) self)
  (Variables|Default|SetPlayer _asfirst_person_character)
  (Utilities|Time|SetTimerbyFunctionName self "GetLightIntensity" 0.2 true))

(event OnComponentEndOverlap(LightCollision)
  (params (OverlappedComponent :type Primitive%20Component%20Object%20Reference) (OtherActor :type Actor%20Object%20Reference) (OtherComp :type Primitive%20Component%20Object%20Reference) (OtherBodyIndex :type Integer))
  (bind _asfirst_person_character (Utilities|Casting|CastToFirstPersonCharacter OtherActor))
  (Utilities|Array|RemoveItem (Variables|/Game/Blueprints/Characters/FirstPersonCharacter/FirstPersonCharacter.FirstPersonCharacter_C|GetActiveLights _asfirst_person_character) self)
  (Utilities|Time|ClearTimerbyFunctionName self "GetLightIntensity")
  (Variables|Default|SetPlayer 0))

(event Custom|GetLightIntensity
  (bind _player (Variables|Default|GetPlayer))
  (bind _pointlight (Variables|Default|GetPointLight))
  (bind _returnvalue (Transformation|GetDistanceTo _player))
  (bind _outhit (Collision|LineTraceByChannel (Transformation|GetActorLocation) (Transformation|GetActorLocation (Variables|Default|GetPlayer)) "TraceTypeQuery2" false 0 "None"))
  (if (== (.hitactor _outhit) _player)
    (bind _output_get (Variables|Default|SetBrightness (* (|(numerator/((pow(distance,2))+1)) (|(pow((clamp((1-(pow((distance/radius),4))),0,1)),2)) _returnvalue (Variables|/Script/Engine.LocalLightComponent|GetAttenuationRadius _pointlight)) _returnvalue) (Variables|/Script/Engine.LightComponentBase|GetIntensity _pointlight))))
    (Development|PrintString (Utilities|String|ToString(Float) _output_get))
    (else
      (Variables|Default|SetBrightness 0.0))))

(fn ConstructionScript
  (bind _pointlight (Variables|Default|GetPointLight))
  (Rendering|Components|Light|SetIntensity _pointlight (Variables|LightConstruction|GetLightIntensity))
  (Rendering|Lighting|SetAttenuationRadius _pointlight (Variables|LightConstruction|GetLightAttenuationRadius))
  (Rendering|Components|Light|SetLightColor _pointlight (Variables|LightConstruction|GetLightColor) true)
  (Components|Sphere|SetSphereRadius (Variables|Default|GetLightCollision) (Variables|/Script/Engine.LocalLightComponent|GetAttenuationRadius (Variables|Default|GetPointLight)) true))