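; Arrow projectile that, on hit, leaves a StaticArrow in its place, notifies AI perception and destroys itself.
; For characters, a short forward Camera-channel trace finds the bone and attaches the arrow there, spawning none if no bone is found.
; Other hits spawn it slightly forward, unattached.
; Every hit reports noise and damage sense events, using the spawn location cached at construction as the damage origin.
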(event Collision|EventHit
  (params (MyComp :type Primitive%20Component%20Object%20Reference) (Other :type Actor%20Object%20Reference) (OtherComp :type Primitive%20Component%20Object%20Reference) (bSelfMoved :type Boolean) (HitLocation :type Vector :default "0, 0, 0") (HitNormal :type Vector :default "0, 0, 0") (NormalImpulse :type Vector :default "0, 0, 0") (Hit :type Hit%20Result%20Structure%20%28by%20ref%29))
  (bind _returnvalue (Transformation|GetActorTransform))
  (bind _returnvalue_2 (Transformation|GetActorTransform))
  (bind _returnvalue_3 (Game|GetInstigator))
  (bind _returnvalue_4 (Math|Vector|GetForwardVector (.rotation _returnvalue)))
  (Variables|Default|SetHitActor Other)
  (Utilities|FlowControl|Sequence
    (:then_0
      ;[1 1 1] Spawn LandedArrow
      (Utilities|Casting|CastToCharacter (Variables|Default|GetHitActor)
        (:then
          (bind (_outhit _returnvalue_5) (Collision|LineTraceByChannel (.location _returnvalue) (+ (.location _returnvalue) (* _returnvalue_4 2e+02)) "TraceTypeQuery2" false 0 "None"))
          (if (and (Utilities|Name|NotEqual(Name) (.hitbonename _outhit) "None") _returnvalue_5)
            (bind _returnvalue_6 (Game|SpawnActorfromClass "/Game/Blueprints/Projectiles/StaticArrow.StaticArrow_C" (Math|Transform|MakeTransform (.location _outhit) (.rotation _returnvalue_2) (.scale _returnvalue_2)) "AlwaysSpawn" 0 0))
            (Transformation|AttachActorToActor _returnvalue_6 (.hitactor _outhit) (.hitbonename _outhit) "KeepWorld" "KeepWorld" "KeepWorld" true)))
        (:CastFailed
          (Game|SpawnActorfromClass "/Game/Blueprints/Projectiles/StaticArrow.StaticArrow_C" (Math|Transform|MakeTransform (+ (* _returnvalue_4 1e+01) (.location _returnvalue)) (.rotation _returnvalue) (.scale _returnvalue)) "AlwaysSpawn" 0 0))))
    (:then_1
      ;[1 1 1] Noise and Damage events
      (Class|AISenseHearing|ReportNoiseEvent HitLocation 1.0 _returnvalue_3 5e+02 "BulletCollision")
      (Class|AISenseDamage|ReportDamageEvent Other _returnvalue_3 2.0 (Variables|Default|GetSpawnLocation) HitLocation))
    (:then_2
      ;[1 1 1] Destroy the Actor
      (Actor|DestroyActor))))

(fn ConstructionScript
  (Variables|/Script/Engine.ProjectileMovementComponent|SetInitialSpeed (Variables|Default|GetProjectile) (Variables|Default|GetProjectileSpeed))
  (Variables|Default|SetSpawnLocation (Transformation|GetActorLocation)))