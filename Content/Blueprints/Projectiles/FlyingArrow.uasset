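; Arrow projectile that turns into a LandedArrow actor when it hits something.
; The construction script applies ProjectileSpeed as the initial speed and records the spawn location.
; On hit it spawns the landed arrow slightly forward along its heading, then destroys itself.
; It also reports an AI damage-sense event with the launch point as event location, without applying damage itself.
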(event Collision|EventHit
  (params (MyComp :type Primitive%20Component%20Object%20Reference) (Other :type Actor%20Object%20Reference) (OtherComp :type Primitive%20Component%20Object%20Reference) (bSelfMoved :type Boolean) (HitLocation :type Vector :default "0, 0, 0") (HitNormal :type Vector :default "0, 0, 0") (NormalImpulse :type Vector :default "0, 0, 0") (Hit :type Hit%20Result%20Structure%20%28by%20ref%29))
  (bind _returnvalue (Transformation|GetActorTransform))
  (Game|SpawnActorfromClass "/Game/Blueprints/Projectiles/LandedArrow.LandedArrow_C" (Math|Transform|MakeTransform (+ (* (Math|Vector|GetForwardVector (.rotation _returnvalue)) 1e+01) (.location _returnvalue)) (.rotation _returnvalue) (.scale _returnvalue)) "AlwaysSpawn" 0 0)
  (Utilities|FlowControl|Sequence
    (:then_0
      (Class|AISenseDamage|ReportDamageEvent Other (Game|GetInstigator) 1e+01 (Variables|Default|GetSpawnLocation) (Transformation|GetActorLocation))
      (Actor|DestroyActor))
    (:then_1
      (Actor|DestroyActor))))

(fn ConstructionScript
  (Variables|/Script/Engine.ProjectileMovementComponent|SetInitialSpeed (Variables|Default|GetProjectile) (Variables|Default|GetProjectileSpeed))
  (Variables|Default|SetSpawnLocation (Transformation|GetActorLocation)))